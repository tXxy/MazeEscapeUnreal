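; BP_Puzzle is a rotation-code puzzle actor linked to a Door.
; CheckCode compares the yaw of three static meshes to a Code array, then calls OpenDOOR on any mismatch and CloseDoor when all match.
; Rotate holds logic to yaw a component and run CheckCode, but it is disconnected from the function entry.
; The event graph, construction script and two other functions do nothing.
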(event EventBeginPlay)

(event Collision|EventActorBeginOverlap
  (params (OtherActor :type Actor%20Object%20Reference)))

(event EventTick
  (params (DeltaSeconds :type Float%20%28single-precision%29)))

(fn ConstructionScript)

(fn Rotate
  (params (Component :type Primitive%20Component%20Object%20Reference)))

(fn CheckCode
  (bind _door (Variables|Default|GetDoor))
  (Utilities|Array|Clear (Variables|Default|GetCodeIsGood))
  (for (_array_element _array_index) (Utilities|Array|MakeArray (.yaw (Variables|/Script/Engine.SceneComponent|GetRelativeRotation (Variables|Default|GetStaticMesh))) (.yaw (Variables|/Script/Engine.SceneComponent|GetRelativeRotation (Variables|Default|GetStaticMesh1))) (.yaw (Variables|/Script/Engine.SceneComponent|GetRelativeRotation (Variables|Default|GetStaticMesh2))))
    (Utilities|Array|Add (Variables|Default|GetCodeIsGood) (Math|Float|NearlyEqual(Float) _array_element (Utilities|Array|Get(acopy) (Variables|Default|GetCode) _array_index) 1e-06)))
  (bind _array_element_2 (Utilities|Array|ForEachLoopwithBreak (Variables|Default|GetCodeIsGood) :!label _label)
    (:LoopBody
      (if (not _array_element_2)
        (LocalVariables|SetLocal%20Failed true)
        (goto _label)))
    (:Completed
      (if (LocalVariables|GetLocal%20Failed)
        (Default|OpenDOOR _door)
        (else
          (Default|CloseDoor _door))))))

(fn NewFunction0
  (params (self2 :type Scene%20Component%20Object%20Reference)))

(fn NewFunction1
  (params (slef2 :type Scene%20Component%20Object%20Reference)))