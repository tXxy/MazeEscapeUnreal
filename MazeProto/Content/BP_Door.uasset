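; BP_Door is a door actor that swings open and closed by rotating its static mesh.
; Open_DOOR plays DoorTimeline and CloseDoor reverses it, with the timeline's ZAxis track setting the mesh's world yaw on each update.
; The yaw is absolute with zero pitch and roll: DefaultRotation is saved at BeginPlay, but the node combining it with the timeline value is unused.
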(event Custom|Open_DOOR
  (bind _zaxis (Timeline|DoorTimeline Play)
    (:Update
      (Transformation|SetWorldRotation (Variables|Debug|GetStaticMeshComponent) (Math|Rotator|MakeRotator 0.0 0.0 _zaxis) false false))))

(event Custom|CloseDoor
  (bind _zaxis (Timeline|DoorTimeline Reverse)
    (:Update
      (Transformation|SetWorldRotation (Variables|Debug|GetStaticMeshComponent) (Math|Rotator|MakeRotator 0.0 0.0 _zaxis) false false))))

(event EventBeginPlay
  (Variables|Default|SetDefaultRotation (Transformation|GetWorldRotation (Variables|Debug|GetStaticMeshComponent))))

(fn ConstructionScript)