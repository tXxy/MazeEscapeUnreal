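; Locked door actor that slides open when the player interacts while holding a key, and plays a closed-door sound otherwise.
; Box overlap with FPCharacter_Kosma stores the character, enables input and opens a Gate, while leaving disables input and closes it.
; With HasKey set, Interact passes the Gate and plays a Timeline that uses VInterpTo to ease the Sciana component toward the Billboard's location, which serves as the target marker.
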(event OnComponentBeginOverlap(Box)
  (params (OverlappedComponent :type Primitive%20Component%20Object%20Reference) (OtherActor :type Actor%20Object%20Reference) (OtherComp :type Primitive%20Component%20Object%20Reference) (OtherBodyIndex :type Integer) (bFromSweep :type Boolean) (SweepResult :type Hit%20Result%20Structure%20%28by%20ref%29))
  (bind _sciana (Variables|Default|Getsciana))
  (bind _asfpcharacter_kosma (Utilities|Casting|CastToFPCharacter_Kosma OtherActor))
  (Input|EnableInput (Game|GetPlayerController 0))
  (Utilities|FlowControl|Gate true) ; enters at Open
)

(event OnComponentEndOverlap(Box)
  (params (OverlappedComponent :type Primitive%20Component%20Object%20Reference) (OtherActor :type Actor%20Object%20Reference) (OtherComp :type Primitive%20Component%20Object%20Reference) (OtherBodyIndex :type Integer))
  (bind _sciana (Variables|Default|Getsciana))
  (Utilities|Casting|CastToFPCharacter_Kosma OtherActor)
  (Input|DisableInput (Game|GetPlayerController 0))
  (Utilities|FlowControl|Gate true) ; enters at Close
)

(event Input|ActionEvents|InputActionInteract
  (params (Key :type Key%20Structure :default "None"))
  (bind _sciana (Variables|Default|Getsciana))
  (:Pressed
    (if (Variables|/Game/BP_Damian/FPCharacter_Kosma.FPCharacter_Kosma_C|GetHasKey? (stale OnComponentBeginOverlap(Box) _asfpcharacter_kosma))
      (Utilities|FlowControl|Gate true
        (:Exit
          (bind _newtrack_0 (Timeline|Timeline_0 Play)
            (:Update
              (Transformation|SetWorldLocation _sciana (Math|Interpolation|VInterpTo (Transformation|GetWorldLocation _sciana) (Transformation|GetWorldLocation (Variables|Default|GetBillboard)) _newtrack_0 0.01) false false)))))
      (else
        (Audio|PlaySoundatLocation "/Game/BP_Damian/closed_doors.closed_doors" (Transformation|GetActorLocation) "0, 0, 0" 1.0 1.0 0.0 0 0 0)))))

(fn ConstructionScript)