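; BP_Puzzle is a rotation-code puzzle that opens or closes Sciana depending on the orientation of three static meshes.
; InterractwithPuzzle yaws the passed component by RotateValue through the Rotate function.
; CheckCode compares each mesh's relative yaw to its Code entry within a fixed tolerance, opening Sciana only if all match.
; Nothing here calls CheckCode, and the Door calls are disconnected.
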(event EventInterractwithPuzzle
  (params (Component :type Primitive%20Component%20Object%20Reference) (Rotate%20Right :type Boolean))
  (CallFunction|Rotate Component))

(fn ConstructionScript)

(fn Rotate
  (params (Component :type Primitive%20Component%20Object%20Reference))
  (Transformation|AddRelativeRotation Component (Math|Rotator|MakeRotator 0.0 0.0 (Variables|Default|GetRotateValue)) false false))

(fn CheckCode
  (bind _sciana (Variables|Default|Getsciana))
  ;[1 1 1] Check code
  (Utilities|Array|Clear (Variables|Default|GetCodeIsGood))
  (for (_array_element _array_index) (Utilities|Array|MakeArray (.yaw (Variables|/Script/Engine.SceneComponent|GetRelativeRotation (Variables|Default|GetStaticMesh))) (.yaw (Variables|/Script/Engine.SceneComponent|GetRelativeRotation (Variables|Default|GetStaticMesh1))) (.yaw (Variables|/Script/Engine.SceneComponent|GetRelativeRotation (Variables|Default|GetStaticMesh2))))
    (Utilities|Array|Add (Variables|Default|GetCodeIsGood) (Math|Float|NearlyEqual(Float) _array_element (Utilities|Array|Get(acopy) (Variables|Default|GetCode) _array_index) 2e+01)))
  (bind _array_element_2 (Utilities|Array|ForEachLoopwithBreak (Variables|Default|GetCodeIsGood) :!label _label)
    (:LoopBody
      (if (not _array_element_2)
        (LocalVariables|SetLocal%20Failed true)
        (goto _label Break)))
    (:Completed
      (if (LocalVariables|GetLocal%20Failed)
        (Default|CloseSciana _sciana)
        (else
          (Default|OpenSciana _sciana))))))

(fn NewFunction0
  (params (self2 :type Scene%20Component%20Object%20Reference)))

(fn NewFunction1
  (params (slef2 :type Scene%20Component%20Object%20Reference)))